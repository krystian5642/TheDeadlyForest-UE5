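; Basic zombie character Blueprint that drives its ABP_ZombieBasic animation instance, cached on BeginPlay.
; Every tick it sends the animation Blueprint its signed forward speed, taken from velocity dotted with the forward vector.
; The death event stops both attack montages and compares facing with the horizontal last shot direction to set a front-hit flag.
; It passes that flag and the alive state on, unless that direction has zero length.
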(event EventBeginPlay
  (bind _asabp_zombie_basic (Utilities|Casting|CastToABP_ZombieBasic (Components|SkeletalMesh|GetAnimInstance (Variables|Character|GetMesh))))
  (Variables|Default|SetAnimation _asabp_zombie_basic))

(event EventTick
  (params (DeltaSeconds :type Float%20%28single-precision%29))
  (Utilities|FlowControl|Sequence
    (:then_0
      (|SetAnimationZombieSpeed))))

(event EventSetAnimationZombieDeath
  (bind _returnvalue (Transformation|GetActorForwardVector))
  (bind _lastshotdirection (Variables|Default|GetLastShotDirection))
  (bind _animation (Variables|Default|GetAnimation))
  (bind _returnvalue_2 (Math|Vector|VectorLength _returnvalue))
  (bind _returnvalue_3 (Math|Vector|MakeVector (.x _lastshotdirection) (.y _lastshotdirection) 0.0))
  (bind _returnvalue_4 (Math|Vector|VectorLength _returnvalue_3))
  (bind _returnvalue_5 (* _returnvalue_2 _returnvalue_4))
  (Animation|StopAnimMontage "/Game/MixamoAnimations/Zombie/Montages/Zombie_Attack_Montage1.Zombie_Attack_Montage1")
  (Animation|StopAnimMontage "/Game/MixamoAnimations/Zombie/Montages/Zombie_Attack_Montage2.Zombie_Attack_Montage2")
  (if (!= _returnvalue_5 0.0)
    (if (> (Class|KismetMathLibrary|DegAcos (/ (Math|Vector|DotProduct _returnvalue _returnvalue_3) _returnvalue_5)) 9e+01)
      (Variables|Default|SetIsFrontHit false)
      (else
        (Variables|Default|SetIsFrontHit true)))
    (Class|BPIAnimationZombie|GetIsFrontHit(Message) _animation (Variables|Default|GetIsFrontHit))
    (Class|BPIAnimationZombie|IsZombieAlive(Message) _animation (Class|BasicZombie|IsAlive))))

(fn ConstructionScript)