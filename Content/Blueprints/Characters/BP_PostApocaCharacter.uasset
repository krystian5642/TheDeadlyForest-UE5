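; Post-apocalyptic player character that takes damage from attacking zombies on overlap and toggles a pause menu.
; Each tick it passes the left-hand transform and aiming state to its cached animation blueprint, which is also messaged on death.
; AdjustMaxWalkSpeed eases walk speed toward a per-movement-mode target with Lerp.
; The pause input flip-flops the widget created at BeginPlay, along with game pause, input mode and cursor.
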(event EventPlayerHasDied
  (Class|BPIAnimationPlayerCharacter|PlayerHasDied(Message) (Variables|Default|GetAnimation) (not (Class|PostApocaCharacter|IsAlive)))
  (Development|PrintString "Hello"))

(event EventBeginPlay
  (bind _asabp_post_apoca_character (Utilities|Casting|CastToABP_PostApocaCharacter (Components|SkeletalMesh|GetAnimInstance (Variables|Character|GetMesh))))
  (Variables|Default|SetAnimation _asabp_post_apoca_character)
  (bind _returnvalue (UserInterface|CreateWidget "/Game/UI/WBP_Pause_Menu.WBP_Pause_Menu_C"))
  (Variables|Default|SetPauseMenu _returnvalue))

(event EventAdjustMaxWalkSpeed
  (bind _output_get (Variables|Default|SetTargetSpeed (Utilities|Select :Index (Variables|Default|GetBasicMovementMode) :Standing 1.5e+02 :Walking 1.5e+02 :Running 4.5e+02 :Aiming 1.5e+02)))
  (bind _output_get_2 (Variables|/Script/Engine.CharacterMovementComponent|SetMaxWalkSpeed (Variables|Character|GetCharacterMovement) (Math|Float|Lerp (stale _output_get_2) _output_get 0.1))))

(event EventTick
  (params (DeltaSeconds :type Float%20%28single-precision%29))
  (bind _animation (Variables|Default|GetAnimation))
  (Utilities|IsValid _animation
    (:Is%20Valid
      (Class|BPIAnimationPlayerCharacter|GetLeftHandTransform(Message) _animation (Variables|Default|GetLeftHandTransform))
      (Class|BPIAnimationPlayerCharacter|IsAiming(Message) _animation (Variables|Default|GetbIsPlayerAiming)))))

(event Collision|EventActorBeginOverlap
  (params (OtherActor :type Actor%20Object%20Reference))
  (bind _asbp_basic_zombie (Utilities|Casting|CastToBP_BasicZombie OtherActor))
  (if (Variables|/Script/TheDeadlyForest.BasicZombie|GetbIsAttacking _asbp_basic_zombie)
    (Class|PostApocaCharacter|TakeDamage (Variables|/Game/Blueprints/Characters/BP_BasicZombie.BP_BasicZombie_C|GetDamage _asbp_basic_zombie) (Utilities|Struct|MakeDamageEvent) (AI|GetAIController _asbp_basic_zombie) _asbp_basic_zombie)))

(event Input|ActionEvents|InputActionPauseGame
  (params (Key :type Key%20Structure :default "None"))
  (bind _returnvalue (Game|GetPlayerController 0))
  (bind _returnvalue_2 (Game|GetPlayerController 0))
  (bind _pausemenu (Variables|Default|GetPauseMenu))
  (:Pressed
    (Utilities|FlowControl|FlipFlop
      (:A
        (UserInterface|Viewport|AddtoViewport _pausemenu 0)
        (Game|SetGamePaused true)
        (Input|SetInputModeGameandUI _returnvalue 0 "DoNotLock" true)
        (Variables|/Script/Engine.PlayerController|SetbShowMouseCursor _returnvalue true))
      (:B
        (Widget|RemovefromParent _pausemenu)
        (Game|SetGamePaused false)
        (Input|SetInputModeGameOnly _returnvalue_2)
        (Variables|/Script/Engine.PlayerController|SetbShowMouseCursor _returnvalue_2 false)))))

(fn ConstructionScript)